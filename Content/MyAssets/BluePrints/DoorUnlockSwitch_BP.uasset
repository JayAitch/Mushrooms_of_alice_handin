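; DoorUnlockSwitch_BP is an overlap switch that locks and unlocks the doors attached to it.
; Each time a ThirdPersonCharacter begins overlapping it, it plays the DoorUnlock sound and flips its ActiveInactive state.
; The MaterialChanger sets the mesh's default material on BeginPlay and receives the new state on each toggle.
; Doors are found through actor attachment, and each attached Door_BP gets a DoorLockUnlock call without being passed the switch's state.
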(event `self.ReceiveBeginPlay`
  ;[1 1 1] Init for material changer
  (`/Game/MyAssets/Components/MaterialChanger.Change Material` (`self.MaterialChanger`) (`self.StaticMeshComponent0`) (`self.DefaultMaterialType`)))

(event `self.ReceiveActorBeginOverlap`
  (params (OtherActor :type "Actor Object Reference"))
  ;[1 1 1] Call unlock on material changer and unlock attached doors
  ;;[1 0.513 0.9064] Check colliding object is character
  (if (== (`GameplayStatics.GetObjectClass` OtherActor) "/Game/ThirdPersonBP/Blueprints/ThirdPersonCharacter.ThirdPersonCharacter_C")
    (`GameplayStatics.PlaySound2D` "/Game/MyAssets/Sound/DoorUnlock.DoorUnlock")
    ;;[0.6543 1 0.5718] Switch material control bool
    (bind _output_get (set `self.ActiveInactive` (not (`self.ActiveInactive`))))
    ;;[1 1 1] Call on material changer
    (`/Game/MyAssets/Components/MaterialChanger.LockingUnlocking` (`self.MaterialChanger`) _output_get)
    ;;[0.5235 0.4331 1] Call Unlock on all attached doors
    (for _array_element (`self.GetAttachedActors`)
      (bind _asdoor_bp (cast `/Game/MyAssets/BluePrints/Door_BP` _array_element))
      (`/Game/MyAssets/BluePrints/Door_BP.DoorLockUnlock` _asdoor_bp))))

(fn `UserConstructionScript`)