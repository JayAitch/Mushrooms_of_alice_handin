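; Bridge container actor that configures its attached Moving_Cuboid actors as one group of moving pieces.
; On BeginPlay it loops over the attached actors, scales each cuboid's own play rate by the container's target rate and passes down the max distance vector.
; The vector's sign alternates by array index, so neighbors in the array get opposite travel offsets before SetMoveSpeed is called on each.
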(event `self.ReceiveBeginPlay`
  ;[1 1 1] Select all attached actors and cast to moving cube
  (for (_array_element _array_index) (`self.GetAttachedActors`)
    (bind _asmoving_cuboid (cast `/Game/MyAssets/BluePrints/Moving_Cuboid` _array_element))
    ;[0.2977 0.3602 1] Set Play rate by a multiple of the components rate
    (bind _output_get (set `self.MovingComponent` _asmoving_cuboid))
    (set `/Game/MyAssets/BluePrints/Moving_Cuboid.PlayRateMod` (* (`self.TargetPlayRate`) (`/Game/MyAssets/BluePrints/Moving_Cuboid.PlayRateMod` _asmoving_cuboid)) _output_get)
    ;[1 0.5521 0.5521] Set relavent movement variables on contained MovingCuboids
    (set `/Game/MyAssets/BluePrints/Moving_Cuboid.LocalMaxDistance` (* (`self.MaxDistance`) (* (`KismetMathLibrary.MultiplyMultiply_FloatFloat` -1.0 (`KismetMathLibrary.Conv_IntToDouble` _array_index)) 1.0)) (`self.MovingComponent`))
    (`/Game/MyAssets/BluePrints/Moving_Cuboid.SetMoveSpeed` (`self.MovingComponent`))))

(fn `UserConstructionScript`)