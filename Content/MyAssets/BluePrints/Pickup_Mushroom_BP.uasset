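; Mushroom pickup actor that spins in place and hands its pickup type to the game instance when the player overlaps it.
; On BeginPlay, a MaterialChanger sets the mushroom mesh material from PickUpType, so the type drives the look.
; Overlap accepts only the exact ThirdPersonCharacter class, plays a sound and calls PickupObject on CustomGI.
; Tick applies RotationSpeed every frame without delta-time scaling.
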(event `self.ReceiveBeginPlay`
  ;[1 1 1] Material change init for data driven materials
  (`/Game/MyAssets/Components/MaterialChanger.Change Material` (`self.MaterialChanger`) (`self.MushroomStaticMesh`) (`self.PickUpType`)))

(event `self.ReceiveActorBeginOverlap`
  (params (OtherActor :type "Actor Object Reference"))
  ;[1 1 1] Collision logic
  (bind _output_get (set `self.CollidingActor` OtherActor))
  ;;[1 0.383 0.5032] Check Colliding actor is player
  (if (== "/Game/ThirdPersonBP/Blueprints/ThirdPersonCharacter.ThirdPersonCharacter_C" (`GameplayStatics.GetObjectClass` _output_get))
    (`GameplayStatics.PlaySound2D` "/Game/MyAssets/Sound/PickUp.PickUp")
    ;;[0.4163 0.4632 1] Send Pickup data to gameinstance
    (bind _ascustom_gi (cast `/Game/Levels/CustomGI` (`GameplayStatics.GetGameInstance`)))
    (`/Game/Levels/CustomGI.PickupObject` _ascustom_gi (`self.PickUpType`) (`self.CollidingActor`))))

(event `self.ReceiveTick`
  (params (DeltaSeconds :type "Float (single-precision)"))
  ;[1 1 1] Simple rotater to rotate pickup
  (`self.K2_SetActorRotation` (`KismetMathLibrary.ComposeRotators` (`self.K2_GetActorRotation`) (`self.RotationSpeed`))))

(fn `UserConstructionScript`)