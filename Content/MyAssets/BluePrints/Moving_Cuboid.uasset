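; Moving cuboid actor that offsets itself from its spawn location along a timeline-driven path.
; On BeginPlay it applies PlayRateMod as the timeline play rate, stores its start location and plays the timeline.
; Each update sets the location to the start plus LocalMaxDistance scaled by the ZMovement track, without sweeping.
; A comment attributes the play rate to an equation on a parent container.
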(event `self.ReceiveBeginPlay`
  ;[1 1 1] Set start location and movespeed
  (`self.SetMoveSpeed`)
  (set `self.StartPosition` (`self.K2_GetActorLocation`))
  (bind (_direction _zmovement) (`Timeline|Movement_Positive_Negative`)
    (:`Update`
      ;[1 1 1] Act on timeline output based on start location
      (`self.K2_SetActorLocation` (+ (`self.StartPosition`) (* (`self.LocalMaxDistance`) _zmovement))))))

(event `SetMoveSpeed`
  ;[1 1 1] Set Timeline play rate from equation on parent container
  (`TimelineComponent.SetPlayRate` (`self.Movement_Positive_Negative`) (`self.PlayRateMod`)))

(fn `UserConstructionScript`)